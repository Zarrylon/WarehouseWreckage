(fn `PrintPropsLeft`
  (params (PropsLeft :type Integer))
  (if (== PropsLeft 0)
    (set `self.PropsText` "You win!!!")
    (else
      (set `self.PropsText` (`KismetTextLibrary.Conv_StringToText` (`KismetStringLibrary.Concat_StrStr` "Props left: " (`KismetStringLibrary.Conv_IntToString` PropsLeft))))))
  (`TextRenderComponent.K2_SetText` (`self.PropsLeft`) (`self.PropsText`)))

(fn `UserConstructionScript`
  (`self.PrintPropsLeft` 0))