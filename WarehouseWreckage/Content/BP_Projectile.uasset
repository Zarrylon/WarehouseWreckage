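; Projectile actor that is launched by a physics impulse and has a configurable lifetime.
; LaunchProjectile applies an Impulse-scaled velocity change to its static mesh along the actor's forward vector.
; BeginPlay starts a one-shot LifeTime timer through a created event, and DestroyProjectile prints the actor's name before destroying it.
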(event `self.ReceiveBeginPlay`
  (`KismetSystemLibrary.K2_SetTimerDelegate` (`|CreateDelegate` :!event `Destroy Projectile`) (`self.Life Time`)))

(fn `Destroy Projectile`
  (`KismetSystemLibrary.PrintString` (`KismetStringLibrary.Concat_StrStr` (`KismetSystemLibrary.GetDisplayName` self) " destroyed"))
  (`self.K2_DestroyActor`))

(fn `Launch Projectile`
  (`PrimitiveComponent.AddImpulse` (`self.StaticMeshComponent`) (* (`self.GetActorForwardVector`) (`self.Impulse`)) "None" true))

(fn `UserConstructionScript`)